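; Basic enemy NPC that runs physical animation on its body and falls into full ragdoll when hit hard enough.
; BeginPlay simulates bones below a named body with motors pulling toward the animation.
; Capsule hits compare both sides' mass-times-speed, and a large difference clears the motor settings and starts ragdoll.
; Ragdoll disables capsule and movement, sets the IsRagdoll blackboard key, and scales joint spring once from bone velocity.
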(event OnComponentHit(CapsuleComponent)
  (params (HitComponent :type Primitive%20Component%20Object%20Reference) (OtherActor :type Actor%20Object%20Reference) (OtherComp :type Primitive%20Component%20Object%20Reference) (NormalImpulse :type Vector :default "0, 0, 0") (Hit :type Hit%20Result%20Structure%20%28by%20ref%29))
  (bind _capsulecomponent (Variables|Default|GetCapsuleComponent))
  (bind _returnvalue (Transformation|GetComponentVelocity _capsulecomponent))
  (bind _returnvalue_2 (Math|Vector|VectorLengthXY _returnvalue))
  (if (< _returnvalue_2 1.0)
    (Variables|Default|SetcurrentVelocity 1.0)
    (else
      (Variables|Default|SetcurrentVelocity _returnvalue_2)))
  (Development|PrintString (Utilities|String|ToString(Float) (Math|Float|Absolute(Float) (- (* (Physics|GetMass OtherComp) (Math|Vector|VectorLengthXY (Transformation|GetVelocity OtherActor))) (* (Variables|Default|GetcurrentVelocity) (Physics|GetMass _capsulecomponent))))) true true "(R=0.000000,G=0.660000,B=1.000000,A=1.000000)" 5.0)
  (if (> (Math|Float|Absolute(Float) (- (* (Physics|GetMass OtherComp) (Math|Vector|VectorLengthXY (Transformation|GetVelocity OtherActor))) (* (Variables|Default|GetcurrentVelocity) (Physics|GetMass _capsulecomponent)))) 3e+04)
    (Class|PhysicalAnimationComponent|ApplyPhysicalAnimationSettingsBelow (Variables|Default|GetPhysicalAnimation) (Variables|Default|GetBody%20Name) (Utilities|Struct|MakePhysicalAnimationData true 0.0) true)
    (CallFunction|StartRagdoll)))

(event OnComponentBeginOverlap(CapsuleComponent)
  (params (OverlappedComponent :type Primitive%20Component%20Object%20Reference) (OtherActor :type Actor%20Object%20Reference) (OtherComp :type Primitive%20Component%20Object%20Reference) (OtherBodyIndex :type Integer) (bFromSweep :type Boolean) (SweepResult :type Hit%20Result%20Structure%20%28by%20ref%29))
  (if (Components|ComponentHasTag OtherComp "HitCollision")
    _))

(event EventBeginPlay
  (Class|PhysicalAnimationComponent|SetSkeletalMeshComponent (Variables|Default|GetPhysicalAnimation) (Variables|Character|GetMesh))
  (Class|PhysicalAnimationComponent|ApplyPhysicalAnimationSettingsBelow (Variables|Default|GetPhysicalAnimation) (Variables|Default|GetBody%20Name) (Utilities|Struct|MakePhysicalAnimationData true 2e+02 0.0 2e+02) true)
  (Class|SkeletalMeshComponent|SetAllBodiesBelowSimulatePhysics (Variables|Character|GetMesh) (Variables|Default|GetBody%20Name) true false)
  (Collision|SetCollisionEnabled (Variables|Default|GetCapsuleComponent) "QueryOnly"))

(event Collision|EventActorBeginOverlap
  (params (OtherActor :type Actor%20Object%20Reference))
  (|CallParentFunction OtherActor))

(event EventTick
  (params (DeltaSeconds :type Float%20%28single-precision%29))
  (|CallParentFunction DeltaSeconds))

(fn ConstructionScript
  (|CallParentFunction))

(fn StartRagdoll
  (bind _mesh (Variables|Character|GetMesh))
  (Utilities|FlowControl|Sequence
    (:then_0
      (Collision|SetCollisionEnabled (Variables|Default|GetCapsuleComponent) "NoCollision")
      (Pawn|Components|CharacterMovement|SetMovementMode (Variables|Character|GetCharacterMovement) "MOVE_None" 0)
      (Collision|SetCollisionObjectType _mesh "ECC_PhysicsBody")
      (Collision|SetCollisionEnabled _mesh "QueryAndPhysics")
      (Class|SkeletalMeshComponent|SetAllBodiesBelowSimulatePhysics (Variables|Character|GetMesh) (Variables|Default|GetBody%20Name) true true)
      (AI|Components|Blackboard|SetValueasBool (AI|GetBlackboard 0) (Utilities|Name|MakeLiteralName "IsRagdoll") true)
      (CallFunction|UpdateRagdoll))))

(fn UpdateRagdoll
  (Class|SkeletalMeshComponent|SetAllMotorsAngularDriveParams (Variables|Character|GetMesh) (Math|Float|MapRangeClamped (Math|Vector|VectorLength (CallFunction|GetRagdollVelocity)) 0.0 0.0 5e+02 1e+01) 0.0 0.0 false))

(fn GetIsRagdoll
  (return (Physics|IsSimulatingPhysics (Variables|Character|GetMesh) (Variables|Default|GetBody%20Name))))

(fn GetRagdollVelocity
  (bind _returnvalue (Class|SkeletalMeshComponent|GetBoneLinearVelocity (Variables|Character|GetMesh) (Variables|Default|GetBody%20Name)))
  (return _returnvalue))