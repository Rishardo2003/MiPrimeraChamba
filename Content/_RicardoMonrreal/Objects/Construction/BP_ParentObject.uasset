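; BP_ParentObject is a base Blueprint for construction objects, with Show and Hide states on a static mesh.
; On BeginPlay it calls Hide, which sets collision to OverlapAll but leaves visibility untouched because that node is disconnected.
; Show makes the mesh visible and sets it to BlockAll.
; The BucketMaterial event and GetBucketMaterial are placeholders: the event's branch does nothing and the getter returns a fixed enum value.
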(event EventBeginPlay
  (CallFunction|Hide))

(event Collision|EventActorBeginOverlap
  (params (OtherActor :type Actor%20Object%20Reference)))

(event EventTick
  (params (DeltaSeconds :type Float%20%28single-precision%29)))

(event EventBucketMaterial
  (params (material :type Bucket_Materials%20Enum :default "NewEnumerator0"))
  (if (Utilities|Enum|Equal(Enum) material "NewEnumerator2")
    _))

(fn ConstructionScript)

(fn Hide
  (Collision|SetCollisionProfileName (Variables|Default|GetStaticMesh) "OverlapAll" true :!class /Script/Engine.PrimitiveComponent))

(fn Show
  (bind _staticmesh (Variables|Default|GetStaticMesh))
  (Rendering|SetVisibility _staticmesh true false)
  (Collision|SetCollisionProfileName _staticmesh "BlockAll" true :!class /Script/Engine.PrimitiveComponent))

(fn GetBucketMaterial
  (return "NewEnumerator0"))