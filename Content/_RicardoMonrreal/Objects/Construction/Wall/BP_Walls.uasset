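; BP_Walls is a construction wall object that counts bricks brought to it and reveals itself once it has enough.
; Each StaticMesh overlap with an actor tagged "Brick" increments CurrentBricks, clamped to BricksNeeded, and calls Show when the count equals that target.
; The overlapping brick is not consumed, and overlaps after completion call Show again.
; Show, Hide, BeginPlay and the construction script only forward to the parent class.
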(event OnComponentBeginOverlap(StaticMesh)
  (params (OverlappedComponent :type Primitive%20Component%20Object%20Reference) (OtherActor :type Actor%20Object%20Reference) (OtherComp :type Primitive%20Component%20Object%20Reference) (OtherBodyIndex :type Integer) (bFromSweep :type Boolean) (SweepResult :type Hit%20Result%20Structure%20%28by%20ref%29))
  (bind _bricksneeded (Variables|Default|GetBricksNeeded))
  (if (Actor|ActorHasTag OtherActor "Brick")
    (bind _output_get (Variables|Default|SetCurrentBricks (Math|Integer|Clamp(Integer) (+ (Variables|Default|GetCurrentBricks) 1) 0 _bricksneeded)))
    (if (== _output_get _bricksneeded)
      (CallFunction|Show))))

(event EventBeginPlay
  (|CallParentFunction))

(event Collision|EventActorBeginOverlap
  (params (OtherActor :type Actor%20Object%20Reference))
  (|CallParentFunction OtherActor) ; This node is disabled and will not be called.\nDrag off pins to build functionality.
)

(event EventTick
  (params (DeltaSeconds :type Float%20%28single-precision%29))
  (|CallParentFunction DeltaSeconds) ; This node is disabled and will not be called.\nDrag off pins to build functionality.
)

(fn ConstructionScript
  (|CallParentFunction))

(fn Hide
  (|CallParentFunction))

(fn Show
  (|CallParentFunction))