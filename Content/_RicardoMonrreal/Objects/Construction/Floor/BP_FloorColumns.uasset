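; BP_FloorColumns is a construction piece for floor columns that starts with a glass material and is built by delivering buckets of mix.
; When a tagged BP_Bucket holding the required material overlaps the mesh, it resets that bucket's material and increments a clamped counter.
; A widget, with show and hide events, displays progress toward MaterialNeed.
; Reaching that target swaps the mesh material and calls the inherited Show.
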(event OnComponentBeginOverlap(StaticMesh)
  (params (OverlappedComponent :type Primitive%20Component%20Object%20Reference) (OtherActor :type Actor%20Object%20Reference) (OtherComp :type Primitive%20Component%20Object%20Reference) (OtherBodyIndex :type Integer) (bFromSweep :type Boolean) (SweepResult :type Hit%20Result%20Structure%20%28by%20ref%29))
  (bind _materialneed (Variables|Default|GetMaterialNeed))
  (Development|PrintString "siessi")
  ;[1 1 1] Comprueba que sea una cubeta con mezcla
  (if (Actor|ActorHasTag OtherActor "Bucket")
    (bind _asbp_bucket (Utilities|Casting|CastToBP_Bucket OtherActor))
    (if (Utilities|Enum|Equal(Enum) (Variables|/Game/_RicardoMonrreal/Objects/Bucket/BP_Bucket.BP_Bucket_C|GetcurrentMaterial _asbp_bucket) "NewEnumerator2")
      (Default|BucketMaterial _asbp_bucket "NewEnumerator0")
      (Class|BPIWidgetInfo|NumMaterial(Message) (UserInterface|GetWidget (Variables|Default|GetWidget)) (Math|Integer|Clamp(Integer) (+ (Variables|Default|GetCurrentMaterials) 1) 0 _materialneed))
      (bind _output_get (Variables|Default|SetCurrentMaterials (Math|Integer|Clamp(Integer) (+ (Variables|Default|GetCurrentMaterials) 1) 0 _materialneed)))
      (if (== _output_get _materialneed)
        (Rendering|Material|SetMaterial (Variables|Default|GetStaticMesh) 0 "/AnimationSharing/AnimSharingBlue.AnimSharingBlue")
        (CallFunction|Show)))))

(event EventBeginPlay
  (|CallParentFunction)
  (Rendering|Material|SetMaterial (Variables|Default|GetStaticMesh) 0 "/DatasmithContent/Materials/FBXImporter/VRED/Glass.Glass")
  (Class|BPIWidgetInfo|SetMaxMaterial(Message) (UserInterface|GetWidget (Variables|Default|GetWidget)) (Variables|Default|GetMaterialNeed)))

(event Collision|EventActorBeginOverlap
  (params (OtherActor :type Actor%20Object%20Reference)))

(event EventTick
  (params (DeltaSeconds :type Float%20%28single-precision%29))
  (|CallParentFunction DeltaSeconds) ; This node is disabled and will not be called.\nDrag off pins to build functionality.
)

(event EventShowWidget
  (Rendering|SetVisibility (Variables|Default|GetWidget) true false))

(event EventHideWidget
  (Rendering|SetVisibility (Variables|Default|GetWidget) false false))

(fn ConstructionScript
  (|CallParentFunction))

(fn Hide
  (|CallParentFunction))

(fn Show
  (|CallParentFunction))

(fn GetBucketMaterial
  (return "NewEnumerator0"))