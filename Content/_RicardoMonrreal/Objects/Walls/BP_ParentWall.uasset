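; Parent Blueprint for a buildable wall that stays hidden and non-blocking until enough bucket loads of mix are delivered.
; When a tagged BP_Bucket holding the required material overlaps the mesh, it resets that bucket's material and increments a clamped concrete count.
; Reaching ConcreteNeeded makes the wall visible and blocking; earlier deliveries print the count.
; Its own BucketMaterial event has no effect, and GetBucketMaterial returns a fixed value.
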(event OnComponentBeginOverlap(StaticMesh)
  (params (OverlappedComponent :type Primitive%20Component%20Object%20Reference) (OtherActor :type Actor%20Object%20Reference) (OtherComp :type Primitive%20Component%20Object%20Reference) (OtherBodyIndex :type Integer) (bFromSweep :type Boolean) (SweepResult :type Hit%20Result%20Structure%20%28by%20ref%29))
  (bind _concreteneeded (Variables|Default|GetConcreteNeeded))
  ;[1 1 1] Comprueba que sea una cubeta con mezcla
  (if (Actor|ActorHasTag OtherActor "Bucket")
    (bind _asbp_bucket (Utilities|Casting|CastToBP_Bucket OtherActor))
    (if (Utilities|Enum|Equal(Enum) (Variables|/Game/_RicardoMonrreal/Objects/Bucket/BP_Bucket.BP_Bucket_C|GetcurrentMaterial _asbp_bucket) "NewEnumerator2")
      (Default|BucketMaterial _asbp_bucket "NewEnumerator0")
      (bind _output_get (Variables|Default|SetCurrentConcrete (Math|Integer|Clamp(Integer) (+ (Variables|Default|GetCurrentConcrete) 1) 0 _concreteneeded)))
      (if (== _output_get _concreteneeded)
        (CallFunction|ShowWall)
        (else
          (Development|PrintString (Utilities|String|ToString(Integer) _output_get)))))))

(event EventBeginPlay
  (CallFunction|HideWall))

(event Collision|EventActorBeginOverlap
  (params (OtherActor :type Actor%20Object%20Reference)))

(event EventTick
  (params (DeltaSeconds :type Float%20%28single-precision%29)))

(event EventBucketMaterial
  (params (material :type Bucket_Materials%20Enum :default "NewEnumerator0"))
  (if (Utilities|Enum|Equal(Enum) material "NewEnumerator2")
    _))

(fn ConstructionScript)

(fn HideWall
  (bind _staticmesh (Variables|Default|GetStaticMesh))
  (Rendering|SetVisibility _staticmesh false false)
  (Collision|SetCollisionProfileName _staticmesh "OverlapAll" true :!class /Script/Engine.PrimitiveComponent))

(fn ShowWall
  (bind _staticmesh (Variables|Default|GetStaticMesh))
  (Rendering|SetVisibility _staticmesh true false)
  (Collision|SetCollisionProfileName _staticmesh "BlockAll" true :!class /Script/Engine.PrimitiveComponent))

(fn GetBucketMaterial
  (return "NewEnumerator0"))