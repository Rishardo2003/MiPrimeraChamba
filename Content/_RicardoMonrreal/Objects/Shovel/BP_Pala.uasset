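; BP_Pala is a shovel actor that visually shows which material, if any, it currently carries.
; The ShovelMaterial event stores an enum state, then either hides the Material mesh component or shows it with a sandstone or rock material.
; GetShovelMaterial returns the stored state.
; Its BeginPlay, overlap and Tick events are disabled stubs.
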(event EventBeginPlay
  (|CallParentFunction) ; This node is disabled and will not be called.\nDrag off pins to build functionality.
)

(event Collision|EventActorBeginOverlap
  (params (OtherActor :type Actor%20Object%20Reference))
  (|CallParentFunction OtherActor) ; This node is disabled and will not be called.\nDrag off pins to build functionality.
)

(event EventTick
  (params (DeltaSeconds :type Float%20%28single-precision%29))
  (|CallParentFunction DeltaSeconds) ; This node is disabled and will not be called.\nDrag off pins to build functionality.
)

(event EventShovelMaterial
  (params (material :type Shovel_Materials%20Enum :default "NewEnumerator0"))
  (bind _material (Variables|Default|GetMaterial))
  (bind _material_2 (Variables|Default|GetMaterial))
  (bind _output_get (Variables|Default|SetcurrentMaterial material))
  (Utilities|FlowControl|Sequence
    (:then_0
      (if (Utilities|Enum|Equal(Enum) _output_get "NewEnumerator0")
        (Rendering|SetVisibility (Variables|Default|GetMaterial) false false)))
    (:then_1
      (if (Utilities|Enum|Equal(Enum) _output_get "NewEnumerator1")
        (Rendering|SetVisibility _material_2 true false)
        (Rendering|Material|SetMaterial _material_2 0 "/Game/StarterContent/Materials/M_Rock_Sandstone.M_Rock_Sandstone")))
    (:then_2
      (if (Utilities|Enum|Equal(Enum) _output_get "NewEnumerator2")
        (Rendering|SetVisibility _material true false)
        (Rendering|Material|SetMaterial _material 0 "/Game/StarterContent/Props/Materials/M_Rock.M_Rock")))))

(fn ConstructionScript
  (|CallParentFunction))

(fn GetShovelMaterial
  (return (Variables|Default|GetcurrentMaterial)))