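; BP_Shovel is a shovel object that tracks and displays which material it currently holds.
; The ShovelMaterial event stores an enum value, then hides the Sphere component for the first value or shows it with a sandstone or rock material for the other two.
; GetShovelMaterial exposes the stored value to other Blueprints.
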(event EventBeginPlay)

(event Collision|EventActorBeginOverlap
  (params (OtherActor :type Actor%20Object%20Reference)))

(event EventTick
  (params (DeltaSeconds :type Float%20%28single-precision%29)))

(event EventShovelMaterial
  (params (material :type Shovel_Materials%20Enum :default "NewEnumerator0"))
  (bind _sphere (Variables|Default|GetSphere))
  (bind _sphere_2 (Variables|Default|GetSphere))
  (bind _output_get (Variables|Default|SetcurrentMaterial material))
  (Utilities|FlowControl|Sequence
    (:then_0
      (if (Utilities|Enum|Equal(Enum) _output_get "NewEnumerator0")
        (Rendering|SetVisibility (Variables|Default|GetSphere) false false)))
    (:then_1
      (if (Utilities|Enum|Equal(Enum) _output_get "NewEnumerator1")
        (Rendering|SetVisibility _sphere_2 true false)
        (Rendering|Material|SetMaterial _sphere_2 0 "/Game/StarterContent/Materials/M_Rock_Sandstone.M_Rock_Sandstone")))
    (:then_2
      (if (Utilities|Enum|Equal(Enum) _output_get "NewEnumerator2")
        (Rendering|SetVisibility _sphere true false)
        (Rendering|Material|SetMaterial _sphere 0 "/Game/StarterContent/Props/Materials/M_Rock.M_Rock")))))

(fn ConstructionScript)

(fn GetShovelMaterial
  (return (Variables|Default|GetcurrentMaterial)))