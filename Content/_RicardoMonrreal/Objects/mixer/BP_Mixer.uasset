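; Concrete mixer that turns cement, sand, gravel and water into concrete for a bucket to collect.
; Box overlaps detect tagged cement, shovels and buckets, exchange materials through message calls, and show the status widget while the player is inside.
; Interact flip-flops the mixer on or off, starting a looping one-second countdown only if all ingredients are present.
; Switching off resets the countdown; completion clears the ingredients and flags concrete ready.
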(event OnComponentBeginOverlap(Box)
  (params (OverlappedComponent :type Primitive%20Component%20Object%20Reference) (OtherActor :type Actor%20Object%20Reference) (OtherComp :type Primitive%20Component%20Object%20Reference) (OtherBodyIndex :type Integer) (bFromSweep :type Boolean) (SweepResult :type Hit%20Result%20Structure%20%28by%20ref%29))
  (bind _returnvalue (Actor|ActorHasTag OtherActor "Bucket"))
  (Utilities|FlowControl|Sequence
    (:then_0
      (if (not (Variables|Default|GetisConcrete))
        (Utilities|FlowControl|Sequence
          (:then_0
            (if (Actor|ActorHasTag OtherActor "Cement")
              (Variables|Default|SetisCement true)
              (Class|BPIWidgetInfo|UpdateValues(Message) (UserInterface|GetWidget (Variables|Default|GetWidget)) 1 "NewEnumerator0")))
          (:then_1
            (if (Actor|ActorHasTag OtherActor "Shovel")
              (bind _currentmaterial (Class|BPIShovel|GetShovelMaterial(Message) OtherActor))
              (if (Utilities|Enum|Equal(Enum) _currentmaterial "NewEnumerator1")
                (Variables|Default|SetisSand true)
                (Class|BPIWidgetInfo|UpdateValues(Message) (UserInterface|GetWidget (Variables|Default|GetWidget)) 1 "NewEnumerator1")
                (Class|BPIShovel|ShovelMaterial(Message) OtherActor "NewEnumerator0" :!label _label)
                (elif (Utilities|Enum|Equal(Enum) _currentmaterial "NewEnumerator2")
                  (Variables|Default|SetisGrava true)
                  (Class|BPIWidgetInfo|UpdateValues(Message) (UserInterface|GetWidget (Variables|Default|GetWidget)) 1 "NewEnumerator2")
                  (goto _label)))))
          (:then_2
            (if _returnvalue
              (bind _currentmaterial_2 (Class|BPIBucket|GetBucketMaterial(Message) OtherActor))
              (if (Utilities|Enum|Equal(Enum) _currentmaterial_2 "NewEnumerator1")
                (Variables|Default|SetisWater true)
                (Class|BPIWidgetInfo|UpdateValues(Message) (UserInterface|GetWidget (Variables|Default|GetWidget)) 1 "NewEnumerator3")
                (Class|BPIBucket|BucketMaterial(Message) OtherActor "NewEnumerator0")))))
        (elif _returnvalue
          (Class|BPIBucket|BucketMaterial(Message) OtherActor "NewEnumerator2")
          (Variables|Default|SetisConcrete false)
          (Class|BPIWidgetInfo|UpdateValues(Message) (UserInterface|GetWidget (Variables|Default|GetWidget)) 0 "NewEnumerator4"))))
    (:then_1
      (if (Actor|ActorHasTag OtherActor "Player")
        (Rendering|SetVisibility (Variables|Default|GetWidget) true false)))))

(event OnComponentEndOverlap(Box)
  (params (OverlappedComponent :type Primitive%20Component%20Object%20Reference) (OtherActor :type Actor%20Object%20Reference) (OtherComp :type Primitive%20Component%20Object%20Reference) (OtherBodyIndex :type Integer))
  (if (Actor|ActorHasTag OtherActor "Player")
    (Rendering|SetVisibility (Variables|Default|GetWidget) false false)))

(event Custom|CustomEvent
  (if (<= (Variables|Default|GetcurrentTimer) 0.0)
    (Variables|Default|SetisSand false)
    (Variables|Default|SetisCement false)
    (Variables|Default|SetisGrava false)
    (Variables|Default|SetisWater false)
    (Variables|Default|SetisConcrete true)
    (Utilities|Time|ClearandInvalidateTimerbyHandle (stale EventInteractFunction _returnvalue))
    (Variables|Default|SetcurrentTimer (Variables|Default|GetmaxTimer))
    (Class|BPIWidgetInfo|UpdateValues(Message) (UserInterface|GetWidget (Variables|Default|GetWidget)) 0 "NewEnumerator0")
    (Class|BPIWidgetInfo|UpdateValues(Message) (UserInterface|GetWidget (Variables|Default|GetWidget)) 0 "NewEnumerator1")
    (Class|BPIWidgetInfo|UpdateValues(Message) (UserInterface|GetWidget (Variables|Default|GetWidget)) 0 "NewEnumerator2")
    (Class|BPIWidgetInfo|UpdateValues(Message) (UserInterface|GetWidget (Variables|Default|GetWidget)) 0 "NewEnumerator3")
    (Class|BPIWidgetInfo|UpdateValues(Message) (UserInterface|GetWidget (Variables|Default|GetWidget)) 1 "NewEnumerator4")
    (CallFunction|ResetTimer)
    (else
      (bind _output_get (Variables|Default|SetcurrentTimer (- (Variables|Default|GetcurrentTimer) 1.0)))
      (Class|BPIWidgetInfo|UpdateTimer(Message) (UserInterface|GetWidget (Variables|Default|GetWidget)) _output_get)
      (if (not (Variables|Default|GetState))
        (Utilities|Time|ClearandInvalidateTimerbyHandle (stale EventInteractFunction _returnvalue))
        (CallFunction|ResetTimer)))))

(event EventBeginPlay
  (Variables|Default|SetisSand false)
  (Variables|Default|SetisCement false)
  (Variables|Default|SetisGrava false)
  (Variables|Default|SetisWater false)
  (CallFunction|ResetTimer))

(event Collision|EventActorBeginOverlap
  (params (OtherActor :type Actor%20Object%20Reference)))

(event EventTick
  (params (DeltaSeconds :type Float%20%28single-precision%29)))

(event EventInteractFunction
  (Utilities|FlowControl|FlipFlop
    (:A
      (Variables|Default|SetState true)
      (if (and (and (and (Variables|Default|GetisCement) (Variables|Default|GetisGrava)) (and (Variables|Default|GetisSand) (Variables|Default|GetisWater))) (Variables|Default|GetState))
        (bind _returnvalue (Utilities|Time|SetTimerbyEvent (delegate Custom|CustomEvent) 1.0 true))))
    (:B
      (Variables|Default|SetState false))))

(fn ConstructionScript)

(fn ResetTimer
  (bind _output_get (Variables|Default|SetcurrentTimer (Variables|Default|GetmaxTimer)))
  (Class|BPIWidgetInfo|UpdateTimer(Message) (UserInterface|GetWidget (Variables|Default|GetWidget)) _output_get))

(fn GetBucketMaterial
  (return "NewEnumerator0"))

(fn GetShovelMaterial
  (return "NewEnumerator0"))