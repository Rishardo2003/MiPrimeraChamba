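; Basic enemy character that uses physical animation to simulate bodies below a configured bone and picks up buckets in its right hand.
; HitRange overlaps attach a bucket in a specific material state to the hand socket, disabling its physics.
; Tick polls attached actors' material messages to trigger detachment and restore physics.
; Ragdoll functions set a blackboard flag and motor strength, but the momentum-based hit check calling them is disconnected.
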(event OnComponentHit(CapsuleComponent)
  (params (HitComponent :type Primitive%20Component%20Object%20Reference) (OtherActor :type Actor%20Object%20Reference) (OtherComp :type Primitive%20Component%20Object%20Reference) (NormalImpulse :type Vector :default "0, 0, 0") (Hit :type Hit%20Result%20Structure%20%28by%20ref%29)))

(event OnComponentBeginOverlap(CapsuleComponent)
  (params (OverlappedComponent :type Primitive%20Component%20Object%20Reference) (OtherActor :type Actor%20Object%20Reference) (OtherComp :type Primitive%20Component%20Object%20Reference) (OtherBodyIndex :type Integer) (bFromSweep :type Boolean) (SweepResult :type Hit%20Result%20Structure%20%28by%20ref%29))
  (if (Components|ComponentHasTag OtherComp "HitCollision")
    _))

(event OnComponentBeginOverlap(HitRange)
  (params (OverlappedComponent :type Primitive%20Component%20Object%20Reference) (OtherActor :type Actor%20Object%20Reference) (OtherComp :type Primitive%20Component%20Object%20Reference) (OtherBodyIndex :type Integer) (bFromSweep :type Boolean) (SweepResult :type Hit%20Result%20Structure%20%28by%20ref%29))
  (if (Actor|ActorHasTag OtherActor "Bucket")
    (if (not (Variables|Default|GetHasBucket?))
      (bind _asbp_bucket (Utilities|Casting|CastToBP_Bucket OtherActor))
      (if (Utilities|Enum|Equal(Enum) (Variables|/Game/_RicardoMonrreal/Objects/Bucket/BP_Bucket.BP_Bucket_C|GetcurrentMaterial _asbp_bucket) "NewEnumerator2")
        (bind _grabbedactorcomponent (CallFunction|HandObjectAttach "RH_Socket" OtherActor OtherComp))
        (Variables|Default|SetHasBucket? true)))))

(event EventBeginPlay
  (Class|PhysicalAnimationComponent|SetSkeletalMeshComponent (Variables|Default|GetPhysicalAnimation) (Variables|Character|GetMesh))
  (Class|PhysicalAnimationComponent|ApplyPhysicalAnimationSettingsBelow (Variables|Default|GetPhysicalAnimation) (Variables|Default|GetBody%20Name) (Utilities|Struct|MakePhysicalAnimationData true 2e+02 0.0 2e+02) true)
  (Class|SkeletalMeshComponent|SetAllBodiesBelowSimulatePhysics (Variables|Character|GetMesh) (Variables|Default|GetBody%20Name) true false)
  (Collision|SetCollisionEnabled (Variables|Default|GetCapsuleComponent) "QueryOnly"))

(event Collision|EventActorBeginOverlap
  (params (OtherActor :type Actor%20Object%20Reference))
  (|CallParentFunction OtherActor))

(event EventTick
  (params (DeltaSeconds :type Float%20%28single-precision%29))
  (|CallParentFunction DeltaSeconds)
  (for _array_element (Actor|GetAttachedActors true false)
    (bind _material (Class|BPIMaterial|GetMaterial(Message) _array_element))
    (if (Utilities|Enum|Equal(Enum) _material "NewEnumerator0")
      (Transformation|DetachFromActor "KeepWorld" "KeepWorld" "KeepWorld")
      (Physics|SetSimulatePhysics (stale OnComponentBeginOverlap(HitRange) _grabbedactorcomponent) true)
      (Collision|SetCollisionProfileName (stale OnComponentBeginOverlap(HitRange) _grabbedactorcomponent) "PhysicsActor" true :!class /Script/Engine.PrimitiveComponent)
      (Variables|Default|SetHasBucket? false))))

(fn ConstructionScript
  (|CallParentFunction))

(fn StartRagdoll
  (bind _mesh (Variables|Character|GetMesh))
  (Utilities|FlowControl|Sequence
    (:then_0
      (Collision|SetCollisionEnabled (Variables|Default|GetCapsuleComponent) "NoCollision")
      (Pawn|Components|CharacterMovement|SetMovementMode (Variables|Character|GetCharacterMovement) "MOVE_None" 0)
      (Collision|SetCollisionObjectType _mesh "ECC_PhysicsBody")
      (Collision|SetCollisionEnabled _mesh "QueryAndPhysics")
      (Class|SkeletalMeshComponent|SetAllBodiesBelowSimulatePhysics (Variables|Character|GetMesh) (Variables|Default|GetBody%20Name) true true)
      (AI|Components|Blackboard|SetValueasBool (AI|GetBlackboard 0) (Utilities|Name|MakeLiteralName "IsRagdoll") true)
      (CallFunction|UpdateRagdoll))))

(fn UpdateRagdoll
  (Class|SkeletalMeshComponent|SetAllMotorsAngularDriveParams (Variables|Character|GetMesh) (Math|Float|MapRangeClamped (Math|Vector|VectorLength (CallFunction|GetRagdollVelocity)) 0.0 0.0 5e+02 0.0) 0.0 0.0 false))

(fn GetIsRagdoll
  (return (Physics|IsSimulatingPhysics (Variables|Character|GetMesh) (Variables|Default|GetBody%20Name))))

(fn GetRagdollVelocity
  (bind _returnvalue (Class|SkeletalMeshComponent|GetBoneLinearVelocity (Variables|Character|GetMesh) (Variables|Default|GetBody%20Name)))
  (return _returnvalue))

(fn HandObjectAttach
  (params (SocketName :type Name) (OtherActor :type Actor%20Object%20Reference) (OtherComponent :type Primitive%20Component%20Object%20Reference))
  (bind _returnvalue (Transformation|AttachComponentToComponent OtherActor (Variables|Character|GetMesh) SocketName "SnapToTarget" "KeepRelative" "KeepWorld" true))
  (if _returnvalue
    (Physics|SetSimulatePhysics OtherComponent false)
    (Collision|SetCollisionProfileName OtherComponent "CustomGrabbedObjects" true :!class /Script/Engine.PrimitiveComponent)
    (return OtherActor OtherComponent)
    (else
      (return 0 0))))

(fn HandObjectDetach
  (params (AttachedObject :type Actor%20Object%20Reference) (AttachedObjectComponent :type Primitive%20Component%20Object%20Reference))
  (Transformation|DetachFromActor "KeepWorld" "KeepWorld" "KeepWorld")
  (Physics|SetSimulatePhysics AttachedObjectComponent true)
  (Collision|SetCollisionProfileName AttachedObjectComponent "PhysicsActor" true :!class /Script/Engine.PrimitiveComponent)
  (return))