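; BP_Fium is an NPC Blueprint variant that sets its own speed, damage and cooldown on top of a parent class.
; BeginPlay assigns those stats and converts Speed to the movement component's max walk speed with a hundredfold scale, without calling the parent's BeginPlay.
; Overlap, Tick and construction only forward to the parent, so any behavior using these stats lives outside this file.
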(event EventBeginPlay
  (bind _output_get (Variables|Default|SetSpeed 3.5))
  (Variables|/Script/Engine.CharacterMovementComponent|SetMaxWalkSpeed (Variables|Character|GetCharacterMovement) (* _output_get 1e+02))
  (Variables|Default|SetDamage 7.0)
  (Variables|Default|Setcooldown 1.5))

(event Collision|EventActorBeginOverlap
  (params (OtherActor :type Actor%20Object%20Reference))
  (|CallParentFunction OtherActor))

(event EventTick
  (params (DeltaSeconds :type Float%20%28single-precision%29))
  (|CallParentFunction DeltaSeconds))

(fn ConstructionScript
  (|CallParentFunction))