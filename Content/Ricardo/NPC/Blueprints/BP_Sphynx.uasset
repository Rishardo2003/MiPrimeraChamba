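; BP_Sphynx is an NPC character Blueprint that sets up the Sphynx's stats on top of a parent class.
; BeginPlay sets speed, damage and cooldown, derives max walk speed from speed, fills ACHealth to max and writes that value to the HP text.
; BeginPlay makes no parent call, while overlap, Tick and the construction script only forward to the parent.
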(event EventBeginPlay
  (bind _ac_health (Variables|Default|GetAC_Health))
  (bind _output_get (Variables|Default|SetSpeed 1.0))
  (Variables|/Script/Engine.CharacterMovementComponent|SetMaxWalkSpeed (Variables|Character|GetCharacterMovement) (* _output_get 1e+02))
  (Variables|Default|SetDamage 7.0)
  (Variables|Default|Setcooldown 1.0)
  (bind _output_get_2 (Variables|/Game/Renato/ZombieSpawner/AC_Health.AC_Health_C|SetCurrentHealth _ac_health (Variables|/Game/Renato/ZombieSpawner/AC_Health.AC_Health_C|GetMaxHealth _ac_health)))
  (Rendering|Components|TextRender|SetText (Variables|Default|GetHP) (Utilities|Text|ToText(Float) _output_get_2 "HalfToEven")))

(event Collision|EventActorBeginOverlap
  (params (OtherActor :type Actor%20Object%20Reference))
  (|CallParentFunction OtherActor))

(event EventTick
  (params (DeltaSeconds :type Float%20%28single-precision%29))
  (|CallParentFunction DeltaSeconds))

(fn ConstructionScript
  (|CallParentFunction))